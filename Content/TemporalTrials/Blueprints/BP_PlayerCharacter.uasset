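; Player character Blueprint for Temporal Trials that lets the player warp to the past or future.
; BeginPlay creates the WBP_Warp widget, adds it to the viewport and sets game-only input.
; The PastWarp and FutureWarp inputs each use their own FlipFlop to alternate between warping and reverting through that widget.
; A shared IsWarped flag makes a new warp revert to the present and wait briefly first.
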(event `self.ReceiveBeginPlay`
  (bind _returnvalue (`GameplayStatics.GetPlayerController` 0))
  (bind _returnvalue_2 (`|CreateWidget` "/Game/TemporalTrials/Widgets/WBP_Warp.WBP_Warp_C" _returnvalue))
  (bind _output_get (set `self.WarpWidget` _returnvalue_2))
  (`UserWidget.AddToViewport` _output_get 0)
  (`Widget.SetVisibility` _returnvalue_2 "Visible")
  (`WidgetBlueprintLibrary.SetInputMode_GameOnly` _returnvalue))

(event `InputAction|PastWarp`
  (params (Key :type "Key Structure"))
  (bind _warpwidget (`self.WarpWidget`))
  (:`Pressed`
    (`/Engine/EditorBlueprintResources/StandardMacros.FlipFlop`
      (:`A`
        (if (`self.isWarped`)
          (`/Game/TemporalTrials/Widgets/WBP_Warp.RevertToPresent` _warpwidget)
          (`KismetSystemLibrary.Delay` 1.0))
        (`/Game/TemporalTrials/Widgets/WBP_Warp.WarpToPast` _warpwidget)
        (set `self.isWarped` true))
      (:`B`
        (`/Game/TemporalTrials/Widgets/WBP_Warp.RevertToPresent` _warpwidget)
        (set `self.isWarped` false)))))

(event `InputAction|FutureWarp`
  (params (Key :type "Key Structure"))
  (bind _warpwidget (`self.WarpWidget`))
  (:`Pressed`
    (`/Engine/EditorBlueprintResources/StandardMacros.FlipFlop`
      (:`A`
        (if (`self.isWarped`)
          (`/Game/TemporalTrials/Widgets/WBP_Warp.RevertToPresent` _warpwidget)
          (`KismetSystemLibrary.Delay` 1.0))
        (`/Game/TemporalTrials/Widgets/WBP_Warp.WarpToFuture` _warpwidget)
        (set `self.isWarped` true))
      (:`B`
        (`/Game/TemporalTrials/Widgets/WBP_Warp.RevertToPresent` _warpwidget)
        (set `self.isWarped` false)))))

(fn `UserConstructionScript`
  (`parent.UserConstructionScript`))